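; Plank obstacle actor with hit points that can be damaged or repaired one plank at a time.
; Damage and Repair step the clamped health and pass it to ChangeHealth, which fires a health-change event.
; The bound handler shows as many of the five plank meshes as there are health points and sets CanBlock to true at zero health.
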(event Custom|OnHealthChanges_Event
  (if (== (Variables|Default|GetHealthPoints) 0)
    (Variables|Default|SetbCanBlock true))
  (for _array_element (Variables|Default|GetArrayMeshes)
    (Rendering|SetVisibility _array_element false false)
    (for _index (range 0 (- (Variables|Default|GetHealthPoints) 1))
      (Rendering|SetVisibility (Utilities|Array|Get(acopy) (Variables|Default|GetArrayMeshes) _index) true false))))

(event EventBeginPlay
  (Variables|Default|SetArrayMeshes (Utilities|Array|MakeArray (Variables|Default|GetPlank1) (Variables|Default|GetPlank2) (Variables|Default|GetPlank3) (Variables|Default|GetPlank4) (Variables|Default|GetPlank5)))
  (EventDispatchers|BindEventtoOnHealthChanges (delegate Custom|OnHealthChanges_Event))
  (CallFunction|OnHealthChangesEvent))

(event Collision|EventActorBeginOverlap
  (params (OtherActor :type Actor%20Object%20Reference)))

(event EventTick
  (params (DeltaSeconds :type Float%20%28single-precision%29)))

(fn ConstructionScript)

(fn ChangeHealth
  (params (Health%20Points :type Integer))
  (Variables|Default|SetHealthPoints Health%20Points)
  (CallFunction|OnHealthChangesEvent))

(fn Damage
  (CallFunction|ChangeHealth (Math|Integer|Clamp(Integer) (- (Variables|Default|GetHealthPoints) 1) 0 5)))

(fn Repair
  (CallFunction|ChangeHealth (Math|Integer|Clamp(Integer) (+ (Variables|Default|GetHealthPoints) 1) 0 5)))