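; Main character Blueprint that handles aim-down-sights zoom for the equipped weapon.
; Holding the right mouse button switches the view from the first-person camera to the weapon's own ZoomCamera, and releasing it switches back.
; The swap toggles camera component activation, gated by a check on WeaponEquipped, with no Tick or construction logic.
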(event EventTick
  (params (DeltaSeconds :type Float%20%28single-precision%29)))

(event Input|MouseEvents|RightMouseButton
  (params (Key :type Key%20Structure :default "None"))
  (bind _firstpersoncameracomponent (Variables|Default|GetFirstPersonCameraComponent))
  (bind _weaponequipped (Variables|Default|GetWeaponEquipped))
  (bind _zoomcamera (Variables|/Script/Zombies.Weapon|GetZoomCamera _weaponequipped))
  (:Pressed
    (if (!= _weaponequipped 0)
      (Components|Activation|Deactivate _firstpersoncameracomponent)
      (Components|Activation|Activate _zoomcamera false)))
  (:Released
    (if (!= (Variables|Default|GetWeaponEquipped) 0)
      (Components|Activation|Deactivate _zoomcamera)
      (Components|Activation|Activate _firstpersoncameracomponent false))))

(fn ConstructionScript)