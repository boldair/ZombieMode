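; Zombie spawner Blueprint that spawns one wave of zombies when play begins, provided Actor1 is set.
; It sets the game mode's CurrentZombies to e raised to CurrentWave, truncated, and copies that into ZombiesToSpawn.
; A ForLoopDelay macro waits once, then loops inclusively from zero to that count, spawning Actor1 at a GetSpawningPoint location each pass.
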(event EventBeginPlay
  (if (!= (Variables|Default|GetActor_1) 0)
    (bind _aszombies_game_mode (Utilities|Casting|CastToZombiesGameMode (Game|GetGameMode)))
    (bind _output_get (Variables|/Script/Zombies.ZombiesGameMode|SetCurrentZombies _aszombies_game_mode (Math|Float|Truncate (Class|KismetMathLibrary|Exp (Math|Conversions|ToFloat(Integer) (Variables|/Script/Zombies.ZombiesGameMode|GetCurrentWave _aszombies_game_mode))))))
    (bind _output_get_2 (Variables|Default|SetZombiesToSpawn _output_get))
    (Utilities|ForLoopDelay 0 _output_get_2 0.5
      (:LoopBody
        (bind _returnvalue (Class|ZombieSpawn|GetSpawningPoint))
        (Class|ZombieSpawn|SpawnOurActor (Variables|Default|GetActor_1) _returnvalue)))))

(event Collision|EventActorBeginOverlap
  (params (OtherActor :type Actor%20Object%20Reference)))

(event EventTick
  (params (DeltaSeconds :type Float%20%28single-precision%29)))

(fn ConstructionScript)